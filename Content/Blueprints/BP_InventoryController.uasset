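; BP_InventoryController toggles the inventory screen with the OpenInventory input action.
; On press it removes the widget if visible, otherwise creates WB_Inventory when no valid instance exists, caches it and adds it to the viewport.
; ReloadInventory calls LoadInventoryItems on a valid widget through a WB_Inventory cast result, but that cast node sits outside any executed path.
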(event EventBeginPlay)

(event EventTick
  (params (DeltaSeconds :type Float%20%28single-precision%29)))

(event EventReloadInventory
  (Utilities|IsValid (Variables|Default|GetInventory%20Widget)
    (:Is%20Valid
      (Default|LoadInventoryItems (stale _aswb_inventory)))))

(event Input|ActionEvents|InputActionOpenInventory
  (params (Key :type Key%20Structure :default "None"))
  (:Pressed
    (if (Widget|IsVisible (Variables|Default|GetInventory%20Widget))
      (Widget|RemovefromParent (Variables|Default|GetInventory%20Widget))
      (else
        (Utilities|IsValid (Variables|Default|GetInventory%20Widget)
          (:Is%20Valid
            _)
          (:Is%20Not%20Valid
            (bind _returnvalue (UserInterface|CreateWidget "/Game/UI/WB_Inventory.WB_Inventory_C"))
            (Variables|Default|SetInventory%20Widget _returnvalue)))
        (UserInterface|Viewport|AddtoViewport (Variables|Default|GetInventory%20Widget) 0)))))

(fn ConstructionScript)